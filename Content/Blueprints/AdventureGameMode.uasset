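; Game mode for an adventure game that sets up item and character managers and fades the camera in on play.
; BeginPlay resolves the game context, gives its managers a world context, and binds quest, item-state and dialog events.
; The quest delay event prints a three-second countdown, then shows a dialog, while the other handlers only print debug messages.
; FadeIn and FadeOut helpers wrap the player camera manager's fade.
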(event Custom|CustomEvent_0
  (params (AffectedItem :type Inventory%20Item%20Object%20Reference))
  (Development|PrintString "Item State changed.")
  (Development|PrintString (Utilities|GetDisplayName AffectedItem)))

(event Custom|DelayEventHandler
  (Development|PrintString "3")
  (Utilities|FlowControl|Delay 1.0)
  (Development|PrintString "2")
  (Utilities|FlowControl|Delay 1.0)
  (Development|PrintString "1")
  (Utilities|FlowControl|Delay 1.0)
  (Class|AdventurePluginBlueprintLibrary|ShowDialog 0 "/Game/Dialogs/ComplexDialog.ComplexDialog"))

(event Custom|Dialog%20Started
  (params (Dialog :type Dialog%20Graph%20Object%20Reference) (GameContext :type Adventure%20Plugin%20Game%20Context%20Object%20Reference))
  (Development|PrintString "Dialog started"))

(event Custom|Dialog%20Ended
  (params (Dialog :type Dialog%20Graph%20Object%20Reference) (GameContext :type Adventure%20Plugin%20Game%20Context%20Object%20Reference))
  (Development|PrintString "Dialog Ended"))

(event EventBeginPlay
  (bind _returnvalue (Class|AdventurePluginGameContext|ResolveGameContext))
  (bind _dialogcontroller (Variables|/Script/AdventurePluginRuntime.AdventurePluginGameContext|GetDialogController _returnvalue))
  (Class|CombinableObjectManager|SetWorldContext (Variables|/Script/AdventurePluginRuntime.AdventurePluginGameContext|GetItemManager (Class|AdventurePluginGameContext|ResolveGameContext)))
  (Class|CombinableObjectManager|SetWorldContext (Variables|/Script/AdventurePluginRuntime.AdventurePluginGameContext|GetAdventureCharacterManager (Class|AdventurePluginGameContext|ResolveGameContext)))
  (Class|AdventurePluginQuestBlueprintLibrary|BindQuestEvent 0 (Variables|Default|GetDelayEventDefinition) (delegate Custom|DelayEventHandler))
  (CallFunction|Fadein 1.0)
  (EventDispatchers|BindEventtoItemStateChanged (Class|AdventurePluginBlueprintLibrary|GetItem 0 "/Game/Items/ItemShovelPart1.ItemShovelPart1_C") (delegate Custom|CustomEvent_0))
  (EventDispatchers|BindEventtoDialogStarted _dialogcontroller (delegate Custom|Dialog%20Started))
  (EventDispatchers|BindEventtoDialogEnded _dialogcontroller (delegate Custom|Dialog%20Ended)))

(event EventTick
  (params (DeltaSeconds :type Float%20%28single-precision%29)))

(fn ConstructionScript)

(fn Fadein
  (params (Duration :type Float%20%28single-precision%29))
  (CameraFades|StartCameraFade :self (Game|GetPlayerCameraManager 0) :FromAlpha 1.0 :Duration Duration :bHoldWhenFinished true))

(fn FadeOut
  (params (Duration :type Float%20%28single-precision%29))
  (CameraFades|StartCameraFade :self (Game|GetPlayerCameraManager 0) :ToAlpha 1.0 :Duration Duration :bHoldWhenFinished true))