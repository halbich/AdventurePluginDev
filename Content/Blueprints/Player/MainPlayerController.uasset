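; Player controller for a point-and-click adventure, handling world clicks, movement and inventory.
; Activate traces under the cursor and forwards the hit location to the actor's ClickableElementComponent, while ToggleInventory flip-flops the inventory display.
; MoveTo uses SimpleMoveToLocation and stores the destination; Tick fires one-shot MovementStopped listeners once the character halts within XY tolerance of it.
; TryUseOn and TryCombineWith line trace for IUseTarget actors to send UseItemMessage, though only TryUseOn passes the item.
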(event EventBeginPlay)

(event EventTick
  (params (DeltaSeconds :type Float%20%28single-precision%29))
  (bind _returnvalue (Game|GetPlayerCharacter 0))
  (if (and (== (Math|Vector|VectorLength (Transformation|GetVelocity _returnvalue)) 0.0) (Utilities|XYEqual (Transformation|GetActorLocation _returnvalue) (Variables|Default|GetMove%20To%20destination) 1e+02))
    (Default|CallMovementStopped)
    (EventDispatchers|UnbindallEventsfromMovementStopped)))

(event Input|ActionEvents|InputActionToggleInventory
  (params (Key :type Key%20Structure))
  (:Pressed
    (bind _isa (Utilities|FlowControl|FlipFlop)
      (:A
        _)
      (:B
        _))
    (Class|AdventurePluginBlueprintLibrary|ShowInventory (Class|APDevBPLibrary|GetCurrentGameContext) _isa)
    (Variables|Default|SetbShowMouseCursor true) ; TODO This is temporary fix
  ))

(event Input|ActionEvents|InputActionActivate
  (params (Key :type Key%20Structure))
  (bind _hitresult (Game|Player|GetHitResultUnderCursorbyChannel "TraceTypeQuery1" true))
  (bind (_bblockinghit _binitialoverlap _time _distance _location _impactpoint _normal _impactnormal _physmat _hitactor) (Collision|BreakHitResult _hitresult))
  (bind _returnvalue (Actor|GetComponentbyClass _hitactor "/Game/Blueprints/Components/ClickableElementComponent.ClickableElementComponent_C"))
  (:Pressed
    (if _bblockinghit
      (EventDispatchers|UnbindallEventsfromMovementStopped)
      (if (Utilities|IsValid _returnvalue)
        (Default|Click _returnvalue _location)
        (Development|PrintString "Clicked on clickable component")
        (else
          (Development|PrintString "Clicked on a component that does not support clicking")))
      (else
        (Development|PrintString "Did not hit")))))

(fn ConstructionScript)

(fn Moveto
  (params (Target%20location :type Vector))
  (AI|Navigation|SimpleMovetoLocation self Target%20location)
  (Variables|Default|SetMove%20To%20destination Target%20location))

(fn MovetoActor)

(fn TryCombinewith
  (params (Actor%20at%20position :type Vector%202D%20Structure) (With%20Item :type Item%20Definition%20Object%20Reference))
  (bind (_tracestart _traceend) (Utilities|GetLineTracePoints Actor%20at%20position))
  (bind _outhit (Collision|LineTraceByChannel _tracestart _traceend "TraceTypeQuery1" false 0 "Persistent"))
  (if (Utilities|DoesObjectImplementInterface (.HitActor (Collision|BreakHitResult _outhit)) "/Game/Blueprints/IUseTarget.IUseTarget_C")
    (Class|IUseTarget|UseItem(Message) (.HitActor (Collision|BreakHitResult _outhit)))
    (else
      (return (and false (Utilities|DoesObjectImplementInterface (.HitActor (Collision|BreakHitResult _outhit)) "/Game/Blueprints/IUseTarget.IUseTarget_C"))))))

(fn TryUseon
  (params (Actor%20at%20position :type Vector%202D%20Structure) (With%20Item :type Inventory%20Item%20Object%20Reference))
  (bind (_tracestart _traceend) (Utilities|GetLineTracePoints Actor%20at%20position))
  (bind _outhit (Collision|LineTraceByChannel _tracestart _traceend "TraceTypeQuery1" false 0 "Persistent"))
  (if (Utilities|DoesObjectImplementInterface (.HitActor (Collision|BreakHitResult _outhit)) "/Game/Blueprints/IUseTarget.IUseTarget_C")
    (bind _wasused (Class|IUseTarget|UseItem(Message) (.HitActor (Collision|BreakHitResult _outhit)) With%20Item)))
  (return (and _wasused (Utilities|DoesObjectImplementInterface (.HitActor (Collision|BreakHitResult _outhit)) "/Game/Blueprints/IUseTarget.IUseTarget_C"))))