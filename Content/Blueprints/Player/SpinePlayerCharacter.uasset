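; Player character Blueprint that drives a Spine skeleton as the visual representation of an adventure character.
; Each tick it derives idle or moving from velocity, applies any active state override, loops the matching animation on track 0 and flips the skeleton by X velocity.
; The adventure character's events set or clear that override.
; One-shot animations use a fixed Delay hack before reporting completion and resetting.
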(event Custom|PlayAnimationOnceHandler
  (params (AnimationName :type Name))
  (CallFunction|SetAnimationState AnimationName)
  (Utilities|FlowControl|Delay 3.0) ; HACK: We should wait for the duration of the animation
  (Class|AdventureCharacter|AnimationFinished (Variables|Default|GetRepresentedCharacterInstance) AnimationName)
  (CallFunction|ResetAnimationState))

(event Custom|SetAnimationStateHandler
  (params (AnimationName :type Name))
  (CallFunction|SetAnimationState AnimationName))

(event Custom|ResetAnimationStateHandler
  (CallFunction|ResetAnimationState))

(event EventBeginPlay
  (bind _representedcharacter (Variables|Default|GetRepresentedCharacter))
  (bind _returnvalue (Class|AdventurePluginBlueprintLibrary|GetAdventureCharacter 0 _representedcharacter))
  (Variables|Default|SetRepresentedCharacterInstance _returnvalue)
  (EventDispatchers|BindEventtoPlayAnimationOnceEvent _returnvalue (delegate Custom|PlayAnimationOnceHandler))
  (EventDispatchers|BindEventtoSetAnimationStateEvent _returnvalue (delegate Custom|SetAnimationStateHandler))
  (EventDispatchers|BindEventtoResetAnimationStateEvent _returnvalue (delegate Custom|ResetAnimationStateHandler)))

(event Collision|EventActorBeginOverlap
  (params (OtherActor :type Actor%20Object%20Reference)))

(event EventTick
  (params (DeltaSeconds :type Float%20%28single-precision%29))
  (CallFunction|UpdateIsMoving)
  (CallFunction|ApplyAnimationOverrideifActive)
  (CallFunction|UpdateAnimation)
  (CallFunction|UpdateOrientation))

(fn ConstructionScript
  (Class|SpineSkeletonAnimationComponent|AddEmptyAnimation (Variables|Default|GetSkeleton) 0 0.0 0.0))

(fn UpdateOrientation
  (bind _self self)
  (bind _skeleton (Variables|Default|GetSkeleton))
  (bind _returnvalue (Transformation|GetVelocity _self))
  (bind _x (Math|Vector|BreakVector _returnvalue))
  (if (> _x 0.0)
    (Class|SpineSkeletonComponent|SetScaleX _skeleton 1.0)
    (elif (< _x 0.0)
      (Class|SpineSkeletonComponent|SetScaleX _skeleton -1.0))))

(fn UpdateIsMoving
  (if (> (Math|Vector|VectorLength (Transformation|GetVelocity self)) 0.0)
    (Variables|Default|SetAnimationState "NewEnumerator2")
    (else
      (Variables|Default|SetAnimationState "NewEnumerator0"))))

(fn UpdateAnimation
  (bind _skeleton (Variables|Default|GetSkeleton))
  (switch Utilities|FlowControl|Switch|SwitchonEMainPlayerAnimationState (Variables|Default|GetAnimationState)
    (:NewEnumerator0
      (LocalVariables|SetSpineAnimationName "idle"))
    (:NewEnumerator1
      (LocalVariables|SetSpineAnimationName "attack"))
    (:NewEnumerator2
      (LocalVariables|SetSpineAnimationName "walk"))
    (:NewEnumerator3
      (LocalVariables|SetSpineAnimationName "fall")))
  (bind _returnvalue (Class|SpineSkeletonAnimationComponent|GetCurrent (Variables|Default|GetSkeleton)))
  (bind _returnvalue_2 (Class|TrackEntry|GetAnimationName _returnvalue))
  (if (Utilities|Enum|NotEqual(Enum) _returnvalue_2 (LocalVariables|GetSpineAnimationName))
    (Class|SpineSkeletonAnimationComponent|ClearTrack _skeleton)
    (Class|SpineSkeletonAnimationComponent|AddAnimation _skeleton 0 (LocalVariables|GetSpineAnimationName) true 0.0)))

(fn ApplyAnimationOverrideifActive
  (if (Variables|Default|GetAnimationStateOverrideActive)
    (Variables|Default|SetAnimationState (Variables|Default|GetAnimationStateOverride))))

(fn SetAnimationState
  (params (NewParam :type Name))
  (bind _animationstate (CallFunction|AnimationNametoAnimationState NewParam))
  (Variables|Default|SetAnimationStateOverride _animationstate)
  (Variables|Default|SetAnimationStateOverrideActive true))

(fn ResetAnimationState
  (Variables|Default|SetAnimationStateOverrideActive false))

(fn AnimationNametoAnimationState
  (params (AnimationName :type Name))
  (switch name AnimationName
    (:Default
      (Development|PrintString "Invalid animation state")
      (return "NewEnumerator0"))
    (:Idle
      (return "NewEnumerator0"))
    (:Moving
      (return "NewEnumerator2"))
    (:Talking
      (return "NewEnumerator1"))
    (:Frozen
      (return "NewEnumerator3"))))