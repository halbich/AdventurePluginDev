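; Point-and-click world actor for an inventory item that can be examined and picked up.
; Clicking it triggers a move to its MoveToTarget; on arrival the first interaction examines the item and sets Examined.
; Later arrivals add it to the game context's inventory and destroy the actor if pickable, otherwise examine it again.
; UseItem returns the message for using another item on this one.
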(event OnClicked(ClickableElementComponent)
  (params (ClickPosition :type Vector :default "0, 0, 0"))
  (Default|Moveto (Variables|Default|GetClickableElementComponent) (Transformation|GetWorldLocation (Variables|Default|GetMoveToTarget))))

(event OnMovetoSuccessful(ClickableElementComponent)
  (bind _returnvalue (Class|APDevBPLibrary|GetCurrentGameContext))
  (bind _item (Variables|Adventure|GetItem))
  (bind _returnvalue_2 (Class|AdventurePluginBlueprintLibrary|GetItem _returnvalue _item))
  (if (Variables|Default|GetExamined)
    (bind _returnvalue_3 (Class|InventoryItem|IsPickable _returnvalue_2 _returnvalue))
    (if _returnvalue_3
      (bind _returnvalue_4 (Class|InventoryController|GetInventory (Variables|/Script/AdventurePluginRuntime.AdventurePluginGameContext|GetInventoryController _returnvalue)))
      (Class|Inventory|AddItem _returnvalue_4 _returnvalue_2 (Class|APDevBPLibrary|GetCurrentGameContext))
      (Actor|DestroyActor)
      (else
        (Class|InventoryItem|Examine _returnvalue_2 _returnvalue :!label _label)
        (Variables|Default|SetExamined true)))
    (else
      (goto _label))))

(event Collision|EventActorBeginOverlap
  (params (OtherActor :type Actor%20Object%20Reference)))

(event EventTick
  (params (DeltaSeconds :type Float%20%28single-precision%29)))

(fn ConstructionScript)

(fn UseItem
  (params (Item :type Inventory%20Item%20Object%20Reference))
  (bind _wasused (Class|IUseTarget|UseItem(Message) Item (Class|AdventurePluginBlueprintLibrary|GetItem (Class|APDevBPLibrary|GetCurrentGameContext) (Variables|Adventure|GetItem))))
  (return _wasused))