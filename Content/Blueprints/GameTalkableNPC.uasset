(event Custom|OnClicked_Event_0
  (params (ClickPosition :type Vector))
  (Default|Moveto (Variables|Default|GetClickableElementComponent) (Transformation|GetWorldLocation (Variables|Default|GetMoveToTarget))))

(event Custom|OnMoveToSuccessful_Event_0
  (bind _asapdev_game_instance (Utilities|Casting|CastToAPDevGameInstance (Game|GetGameInstance)))
  (Development|PrintString "NPC Clicked")
  (Class|AdventurePluginBlueprintLibrary|ShowDialog (Variables|/Script/AdventurePluginDev.APDevGameInstance|GetCurrentGameContext _asapdev_game_instance) (Variables|Default|GetDialog)))

(event EventBeginPlay
  (bind _clickableelementcomponent (Variables|Default|GetClickableElementComponent))
  (EventDispatchers|AssignOnClicked _clickableelementcomponent (delegate Custom|OnClicked_Event_0))
  (EventDispatchers|AssignOnMovetoSuccessful _clickableelementcomponent (delegate Custom|OnMoveToSuccessful_Event_0)))

(event Collision|EventActorBeginOverlap
  (params (OtherActor :type Actor%20Object%20Reference)))

(event EventTick
  (params (DeltaSeconds :type Float%20%28single-precision%29)))

(fn ConstructionScript)

(fn Combinewith
  (params (OtherItem :type Item%20Definition%20Object%20Reference))
  (return true))

(fn UseItem
  (params (Item :type Inventory%20Item%20Object%20Reference))
  (Development|PrintText (Utilities|Text|FormatText "NPC thanks for the {0}." (Variables|/Script/AdventurePluginRuntime.InventoryItem|GetName Item)))
  (return true))