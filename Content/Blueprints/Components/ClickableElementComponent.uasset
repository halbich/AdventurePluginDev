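; Component for clickable world elements that relays clicks and movement requests between its owner and the player controller.
; Click broadcasts OnClicked with the click position.
; MoveTo sends a target location to MainPlayerController and binds a callback to its movement-stopped event, while MoveToSuccessful rebroadcasts as OnMoveToSuccessful.
; MoveToActor is an empty stub with disconnected movement logic.
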(event Custom|Move%20To%20Successful
  (Default|CallOnMovetoSuccessful))

(event EventBeginPlay)

(event EventTick
  (params (DeltaSeconds :type Float%20%28single-precision%29)))

(fn Click
  (params (ClickPosition :type Vector))
  (Default|CallOnClicked ClickPosition))

(fn Moveto
  (params (Target%20location :type Vector))
  (bind _asmain_player_controller (Utilities|Casting|CastToMainPlayerController (Game|GetPlayerController 0)))
  (Default|Moveto _asmain_player_controller Target%20location)
  (EventDispatchers|BindEventtoMovementStopped _asmain_player_controller (EventDispatchers|CreateEvent :!event Custom|Move%20To%20Successful)))

(fn MovetoActor)