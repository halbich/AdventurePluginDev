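; Component that turns a clickable level exit into a transition to another level.
; On click it moves to a configured walk position, or to the clicked point if that position is zero.
; When the move succeeds, it fades out through AdventureGameMode, waits for the fade, then opens the target level by name.
; The target start position is passed as the level's options string.
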(event Custom|OnMoveToSuccessful_Event_0
  (Development|PrintString "Moved to target")
  (bind _asadventure_game_mode (Utilities|Casting|CastToAdventureGameMode (Game|GetGameMode)))
  (Default|FadeOut _asadventure_game_mode 0.5)
  (Utilities|FlowControl|Delay 0.5)
  (Game|OpenLevel(byName) (Variables|Default|GetTargetLevelName) true (Variables|Default|GetTargetLevelStartPosition)))

(event Custom|OnClicked_Event_0
  (params (ClickPosition :type Vector))
  (bind _walk_to_position (Variables|Default|GetWalk%20to%20position))
  (Development|PrintString "Level end clicked")
  (if (Math|Vector|NotEqual(Vector) _walk_to_position "0, 0, 0" 0.0001)
    (CallFunction|Moveto _walk_to_position)
    (else
      (CallFunction|Moveto ClickPosition))))

(event EventBeginPlay
  (|CallParentFunction)
  (EventDispatchers|AssignOnClicked (delegate Custom|OnClicked_Event_0))
  (EventDispatchers|AssignOnMovetoSuccessful (delegate Custom|OnMoveToSuccessful_Event_0)))

(event EventTick
  (params (DeltaSeconds :type Float%20%28single-precision%29))
  (|CallParentFunction DeltaSeconds) ; This node is disabled and will not be called.\nDrag off pins to build functionality.
)